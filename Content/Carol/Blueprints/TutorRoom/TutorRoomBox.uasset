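; TutorRoomBox is a trigger volume for the tutor room that tracks when the ThirdPersonCharacter is inside and switches the room lights.
; On begin overlap it sets the character's Room to 1, then swaps every LightTutorRoom actor to the on material and raises its point light intensity.
; On end overlap it resets Room to 0, restores the off material and dims those lights.
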(event OnComponentBeginOverlap(TutorRoomBox)
  (params (OverlappedComponent :type Primitive%20Component%20Object%20Reference) (OtherActor :type Actor%20Object%20Reference) (OtherComp :type Primitive%20Component%20Object%20Reference) (OtherBodyIndex :type Integer) (bFromSweep :type Boolean) (SweepResult :type Hit%20Result%20Structure%20%28by%20ref%29))
  (bind _asthird_person_character (Utilities|Casting|CastToThirdPersonCharacter OtherActor))
  (Variables|/Game/ThirdPersonBP/Blueprints/ThirdPersonCharacter.ThirdPersonCharacter_C|SetRoom _asthird_person_character 1)
  (bind _outactors (Actor|GetAllActorsOfClass "/Game/Carol/Blueprints/Lights/LightTutorRoom.LightTutorRoom_C"))
  (for _array_element _outactors
    (Rendering|Material|SetMaterial (Variables|/Game/Carol/Blueprints/Lights/LightTutorRoom.LightTutorRoom_C|GetLight _array_element) 0 "/Game/Carol/Materials/LightOnMaterial.LightOnMaterial")
    (Rendering|Components|Light|SetIntensity (Variables|/Game/Carol/Blueprints/Lights/LightTutorRoom.LightTutorRoom_C|GetPointLight _array_element) 1e+05)))

(event OnComponentEndOverlap(TutorRoomBox)
  (params (OverlappedComponent :type Primitive%20Component%20Object%20Reference) (OtherActor :type Actor%20Object%20Reference) (OtherComp :type Primitive%20Component%20Object%20Reference) (OtherBodyIndex :type Integer))
  (bind _asthird_person_character (Utilities|Casting|CastToThirdPersonCharacter OtherActor))
  (Variables|/Game/ThirdPersonBP/Blueprints/ThirdPersonCharacter.ThirdPersonCharacter_C|SetRoom _asthird_person_character 0)
  (bind _outactors (Actor|GetAllActorsOfClass "/Game/Carol/Blueprints/Lights/LightTutorRoom.LightTutorRoom_C"))
  (for _array_element _outactors
    (Rendering|Material|SetMaterial (Variables|/Game/Carol/Blueprints/Lights/LightTutorRoom.LightTutorRoom_C|GetLight _array_element) 0 "/Game/Carol/Materials/LightOffMaterial.LightOffMaterial")
    (Rendering|Components|Light|SetIntensity (Variables|/Game/Carol/Blueprints/Lights/LightTutorRoom.LightTutorRoom_C|GetPointLight _array_element) 1e+03)))

(event EventBeginPlay)

(event Collision|EventActorBeginOverlap
  (params (OtherActor :type Actor%20Object%20Reference)))

(event EventTick
  (params (DeltaSeconds :type Float%20%28single-precision%29)))

(fn ConstructionScript)