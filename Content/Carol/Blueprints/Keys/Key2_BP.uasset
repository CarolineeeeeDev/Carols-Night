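; Key2_BP is the pickup actor for the second key, which the player collects with E while inside its box.
; Box overlaps with ThirdPersonCharacter toggle the actor's input and a Pick flag.
; On pickup, it writes its Item into a fixed MissionProps slot in the GameInstance inventory, updates the inventory widget, sets GetKey2 on the character and destroys itself.
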(event OnComponentBeginOverlap(Box)
  (params (OverlappedComponent :type Primitive%20Component%20Object%20Reference) (OtherActor :type Actor%20Object%20Reference) (OtherComp :type Primitive%20Component%20Object%20Reference) (OtherBodyIndex :type Integer) (bFromSweep :type Boolean) (SweepResult :type Hit%20Result%20Structure%20%28by%20ref%29))
  (Utilities|Casting|CastToThirdPersonCharacter OtherActor)
  (Input|EnableInput (Game|GetPlayerController 0))
  (Variables|Default|SetPick true))

(event OnComponentEndOverlap(Box)
  (params (OverlappedComponent :type Primitive%20Component%20Object%20Reference) (OtherActor :type Actor%20Object%20Reference) (OtherComp :type Primitive%20Component%20Object%20Reference) (OtherBodyIndex :type Integer))
  (Utilities|Casting|CastToThirdPersonCharacter OtherActor)
  (Input|DisableInput (Game|GetPlayerController 0))
  (Variables|Default|SetPick false))

(event EventBeginPlay)

(event Collision|EventActorBeginOverlap
  (params (OtherActor :type Actor%20Object%20Reference)))

(event EventTick
  (params (DeltaSeconds :type Float%20%28single-precision%29)))

(event Input|KeyboardEvents|E
  (params (Key :type Key%20Structure :default "None"))
  (:Pressed
    (if (Variables|Default|GetPick)
      (bind _asbp_game_instance (Utilities|Casting|CastToBP_GameInstance (Game|GetGameInstance)))
      (Utilities|Array|SetArrayElem (.MissionProps (Utilities|Struct|BreakS_Inventory (Variables|/Game/CarolProject/Blueprints/BP_GameInstance.BP_GameInstance_C|GetInventory _asbp_game_instance))) 1 (Variables|Default|GetItem))
      (bind _asthird_person_character (Utilities|Casting|CastToThirdPersonCharacter (Game|GetPlayerCharacter 0)))
      (Default|SetInventoryItem (Variables|/Game/Carol/UI/Inventory/W_Main.W_Main_C|GetW_Inventory (Variables|/Game/ThirdPersonBP/Blueprints/ThirdPersonCharacter.ThirdPersonCharacter_C|GetUI _asthird_person_character)) "NewEnumerator0")
      (Variables|/Game/ThirdPersonBP/Blueprints/ThirdPersonCharacter.ThirdPersonCharacter_C|SetGetKey2 _asthird_person_character true)
      (Actor|DestroyActor))))

(fn ConstructionScript)