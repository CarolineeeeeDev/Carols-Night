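; Boss room floor that yaws through 360 degrees via a timeline started on BeginPlay and hosts an ordered cube puzzle.
; Seven trigger boxes advance an overlapping CubeBP through button materials, using its current material as progress state so boxes only count in sequence.
; The first box fires only once.
; The last box destroys the cube, spawns a BlackWall and moves the player to a hardcoded location.
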(event OnComponentBeginOverlap(Box1)
  (params (OverlappedComponent :type Primitive%20Component%20Object%20Reference) (OtherActor :type Actor%20Object%20Reference) (OtherComp :type Primitive%20Component%20Object%20Reference) (OtherBodyIndex :type Integer) (bFromSweep :type Boolean) (SweepResult :type Hit%20Result%20Structure%20%28by%20ref%29))
  (bind _ascube_bp (Utilities|Casting|CastToCubeBP OtherActor))
  (Utilities|FlowControl|DoOnce false
    (:Completed
      (Rendering|Material|SetMaterial (Variables|/Game/Carol/Blueprints/BossRoom/CubeBP.CubeBP_C|GetCube _ascube_bp) 0 "/Game/Carol/Materials/Button1Material.Button1Material"))))

(event OnComponentBeginOverlap(Box2)
  (params (OverlappedComponent :type Primitive%20Component%20Object%20Reference) (OtherActor :type Actor%20Object%20Reference) (OtherComp :type Primitive%20Component%20Object%20Reference) (OtherBodyIndex :type Integer) (bFromSweep :type Boolean) (SweepResult :type Hit%20Result%20Structure%20%28by%20ref%29))
  (bind _ascube_bp (Utilities|Casting|CastToCubeBP OtherActor))
  (if (== (Rendering|Material|GetMaterial (Variables|/Game/Carol/Blueprints/BossRoom/CubeBP.CubeBP_C|GetCube _ascube_bp) 0) "/Game/Carol/Materials/Button1Material.Button1Material")
    (Rendering|Material|SetMaterial (Variables|/Game/Carol/Blueprints/BossRoom/CubeBP.CubeBP_C|GetCube _ascube_bp) 0 "/Game/Carol/Materials/Button2Material.Button2Material")))

(event OnComponentBeginOverlap(Box3)
  (params (OverlappedComponent :type Primitive%20Component%20Object%20Reference) (OtherActor :type Actor%20Object%20Reference) (OtherComp :type Primitive%20Component%20Object%20Reference) (OtherBodyIndex :type Integer) (bFromSweep :type Boolean) (SweepResult :type Hit%20Result%20Structure%20%28by%20ref%29))
  (bind _ascube_bp (Utilities|Casting|CastToCubeBP OtherActor))
  (if (== (Rendering|Material|GetMaterial (Variables|/Game/Carol/Blueprints/BossRoom/CubeBP.CubeBP_C|GetCube _ascube_bp) 0) "/Game/Carol/Materials/Button2Material.Button2Material")
    (Rendering|Material|SetMaterial (Variables|/Game/Carol/Blueprints/BossRoom/CubeBP.CubeBP_C|GetCube _ascube_bp) 0 "/Game/Carol/Materials/Button3Material.Button3Material")))

(event OnComponentBeginOverlap(Box4)
  (params (OverlappedComponent :type Primitive%20Component%20Object%20Reference) (OtherActor :type Actor%20Object%20Reference) (OtherComp :type Primitive%20Component%20Object%20Reference) (OtherBodyIndex :type Integer) (bFromSweep :type Boolean) (SweepResult :type Hit%20Result%20Structure%20%28by%20ref%29))
  (bind _ascube_bp (Utilities|Casting|CastToCubeBP OtherActor))
  (if (== (Rendering|Material|GetMaterial (Variables|/Game/Carol/Blueprints/BossRoom/CubeBP.CubeBP_C|GetCube _ascube_bp) 0) "/Game/Carol/Materials/Button3Material.Button3Material")
    (Rendering|Material|SetMaterial (Variables|/Game/Carol/Blueprints/BossRoom/CubeBP.CubeBP_C|GetCube _ascube_bp) 0 "/Game/Carol/Materials/Button4Material.Button4Material")))

(event OnComponentBeginOverlap(Box5)
  (params (OverlappedComponent :type Primitive%20Component%20Object%20Reference) (OtherActor :type Actor%20Object%20Reference) (OtherComp :type Primitive%20Component%20Object%20Reference) (OtherBodyIndex :type Integer) (bFromSweep :type Boolean) (SweepResult :type Hit%20Result%20Structure%20%28by%20ref%29))
  (bind _ascube_bp (Utilities|Casting|CastToCubeBP OtherActor))
  (if (== (Rendering|Material|GetMaterial (Variables|/Game/Carol/Blueprints/BossRoom/CubeBP.CubeBP_C|GetCube _ascube_bp) 0) "/Game/Carol/Materials/Button4Material.Button4Material")
    (Rendering|Material|SetMaterial (Variables|/Game/Carol/Blueprints/BossRoom/CubeBP.CubeBP_C|GetCube _ascube_bp) 0 "/Game/Carol/Materials/Button5Material.Button5Material")))

(event OnComponentBeginOverlap(Box6)
  (params (OverlappedComponent :type Primitive%20Component%20Object%20Reference) (OtherActor :type Actor%20Object%20Reference) (OtherComp :type Primitive%20Component%20Object%20Reference) (OtherBodyIndex :type Integer) (bFromSweep :type Boolean) (SweepResult :type Hit%20Result%20Structure%20%28by%20ref%29))
  (bind _ascube_bp (Utilities|Casting|CastToCubeBP OtherActor))
  (if (== (Rendering|Material|GetMaterial (Variables|/Game/Carol/Blueprints/BossRoom/CubeBP.CubeBP_C|GetCube _ascube_bp) 0) "/Game/Carol/Materials/Button5Material.Button5Material")
    (Rendering|Material|SetMaterial (Variables|/Game/Carol/Blueprints/BossRoom/CubeBP.CubeBP_C|GetCube _ascube_bp) 0 "/Game/Carol/Materials/Button6Material.Button6Material")))

(event OnComponentBeginOverlap(Box7)
  (params (OverlappedComponent :type Primitive%20Component%20Object%20Reference) (OtherActor :type Actor%20Object%20Reference) (OtherComp :type Primitive%20Component%20Object%20Reference) (OtherBodyIndex :type Integer) (bFromSweep :type Boolean) (SweepResult :type Hit%20Result%20Structure%20%28by%20ref%29))
  (bind _ascube_bp (Utilities|Casting|CastToCubeBP OtherActor))
  (if (== (Rendering|Material|GetMaterial (Variables|/Game/Carol/Blueprints/BossRoom/CubeBP.CubeBP_C|GetCube _ascube_bp) 0) "/Game/Carol/Materials/Button6Material.Button6Material")
    (Rendering|Material|SetMaterial (Variables|/Game/Carol/Blueprints/BossRoom/CubeBP.CubeBP_C|GetCube _ascube_bp) 0 "/Game/Carol/Materials/Button7Material.Button7Material")
    (Actor|DestroyActor _ascube_bp)
    (Game|SpawnActorfromClass "/Game/Carol/Blueprints/TutorRoom/BlackWall.BlackWall_C" (Math|Transform|MakeTransform "-1951.311279,4000.777100,815.442444" "0, 0, 0" "14.829773,1,12.530029") "Undefined" 0 0)
    (Transformation|SetActorLocation (Game|GetPlayerCharacter 0) "-1902.360107,5082.343750,961.007996" false false)))

(event EventBeginPlay
  (bind _newtrack_0 (Timeline|FloorRotate Play)
    (:Update
      (Transformation|SetActorRotation (Math|Rotator|MakeRotator 0.0 0.0 (Math|Float|Lerp 0.0 3.6e+02 _newtrack_0))))))

(event Collision|EventActorBeginOverlap
  (params (OtherActor :type Actor%20Object%20Reference)))

(event EventTick
  (params (DeltaSeconds :type Float%20%28single-precision%29)))

(fn ConstructionScript)