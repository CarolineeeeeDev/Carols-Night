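; BinBP is a physics-simulated bin for Room 102 that rewards collecting balls with a key.
; Each Ball that overlaps its Box trigger is destroyed and increments BallCount.
; Tick polls that count and, once it equals nine, uses a DoOnce to play a drop sound and spawn Key3_BP at a hard-coded world location.
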(event OnComponentBeginOverlap(Box)
  (params (OverlappedComponent :type Primitive%20Component%20Object%20Reference) (OtherActor :type Actor%20Object%20Reference) (OtherComp :type Primitive%20Component%20Object%20Reference) (OtherBodyIndex :type Integer) (bFromSweep :type Boolean) (SweepResult :type Hit%20Result%20Structure%20%28by%20ref%29))
  (bind _asball (Utilities|Casting|CastToBall OtherActor))
  (Actor|DestroyActor _asball)
  (Variables|Default|SetBallCount (+ (Variables|Default|GetBallCount) 1)))

(event EventBeginPlay
  (Physics|SetSimulatePhysics (Variables|Default|GetBin) true))

(event Collision|EventActorBeginOverlap
  (params (OtherActor :type Actor%20Object%20Reference)))

(event EventTick
  (params (DeltaSeconds :type Float%20%28single-precision%29))
  (if (== (Variables|Default|GetBallCount) 9)
    (Utilities|FlowControl|DoOnce false
      (:Completed
        (Audio|PlaySoundatLocation "/Game/Carol/Audio/DropKey_Cue.DropKey_Cue" "-30.168625,1369.416016,737.850281" "0, 0, 0" 1.0 1.0 0.0 0 0 0)
        (Game|SpawnActorfromClass "/Game/Carol/Blueprints/Keys/Key3_BP.Key3_BP_C" (Math|Transform|MakeTransform "-30.168625,1369.416016,737.850281") "Undefined" 0 0)))))

(fn ConstructionScript)