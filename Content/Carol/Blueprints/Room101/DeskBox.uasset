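; DeskBox is a trigger in Room101 that changes the look of the blackboards when the ThirdPersonCharacter enters or leaves it.
; On overlap begin, it finds every BlackboardBP actor and sets the first material slot of its Blackboard component to BlackboardMaterial.
; On overlap end, it repeats the search and switches that slot to AllObjectsMaterial.
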(event OnComponentBeginOverlap(DeskBox)
  (params (OverlappedComponent :type Primitive%20Component%20Object%20Reference) (OtherActor :type Actor%20Object%20Reference) (OtherComp :type Primitive%20Component%20Object%20Reference) (OtherBodyIndex :type Integer) (bFromSweep :type Boolean) (SweepResult :type Hit%20Result%20Structure%20%28by%20ref%29))
  (Utilities|Casting|CastToThirdPersonCharacter OtherActor)
  (bind _outactors (Actor|GetAllActorsOfClass "/Game/Carol/Blueprints/Room101/BlackboardBP.BlackboardBP_C"))
  (for _array_element _outactors
    (Rendering|Material|SetMaterial (Variables|/Game/Carol/Blueprints/Room101/BlackboardBP.BlackboardBP_C|GetBlackboard _array_element) 0 "/Game/Carol/Materials/BlackboardMaterial.BlackboardMaterial")))

(event OnComponentEndOverlap(DeskBox)
  (params (OverlappedComponent :type Primitive%20Component%20Object%20Reference) (OtherActor :type Actor%20Object%20Reference) (OtherComp :type Primitive%20Component%20Object%20Reference) (OtherBodyIndex :type Integer))
  (Utilities|Casting|CastToThirdPersonCharacter OtherActor)
  (bind _outactors (Actor|GetAllActorsOfClass "/Game/Carol/Blueprints/Room101/BlackboardBP.BlackboardBP_C"))
  (for _array_element _outactors
    (Rendering|Material|SetMaterial (Variables|/Game/Carol/Blueprints/Room101/BlackboardBP.BlackboardBP_C|GetBlackboard _array_element) 0 "/Game/Carol/Materials/AllObjectsMaterial.AllObjectsMaterial")))

(event EventBeginPlay)

(event Collision|EventActorBeginOverlap
  (params (OtherActor :type Actor%20Object%20Reference)))

(event EventTick
  (params (DeltaSeconds :type Float%20%28single-precision%29)))

(fn ConstructionScript)