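; Portal actor that moves the player to the Portal2BP in the level when a ThirdPersonCharacter enters its Box.
; On overlap, if the character's InPortal flag is clear, player character 0 is placed slightly above that actor's Portal component.
; The character's InPortal flag is set after the move and cleared when it leaves this Box, gating repeat teleports.
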(event OnComponentBeginOverlap(Box)
  (params (OverlappedComponent :type Primitive%20Component%20Object%20Reference) (OtherActor :type Actor%20Object%20Reference) (OtherComp :type Primitive%20Component%20Object%20Reference) (OtherBodyIndex :type Integer) (bFromSweep :type Boolean) (SweepResult :type Hit%20Result%20Structure%20%28by%20ref%29))
  (bind _asthird_person_character (Utilities|Casting|CastToThirdPersonCharacter OtherActor))
  (if (not (Variables|/Game/ThirdPersonBP/Blueprints/ThirdPersonCharacter.ThirdPersonCharacter_C|GetInPortal _asthird_person_character))
    (bind _returnvalue (Actor|GetActorOfClass "/Game/Carol/Blueprints/Room103/Portal2BP.Portal2BP_C"))
    (Transformation|SetActorLocation (Game|GetPlayerCharacter 0) (Math|Vector|MakeVector (.X (Math|Vector|BreakVector (Transformation|GetWorldLocation (Variables|/Game/Carol/Blueprints/Room103/Portal2BP.Portal2BP_C|GetPortal _returnvalue)))) (.Y (Math|Vector|BreakVector (Transformation|GetWorldLocation (Variables|/Game/Carol/Blueprints/Room103/Portal2BP.Portal2BP_C|GetPortal _returnvalue)))) (+ (.Z (Math|Vector|BreakVector (Transformation|GetWorldLocation (Variables|/Game/Carol/Blueprints/Room103/Portal2BP.Portal2BP_C|GetPortal _returnvalue)))) 4e+01)) false false)
    (Variables|/Game/ThirdPersonBP/Blueprints/ThirdPersonCharacter.ThirdPersonCharacter_C|SetInPortal _asthird_person_character true)))

(event OnComponentEndOverlap(Box)
  (params (OverlappedComponent :type Primitive%20Component%20Object%20Reference) (OtherActor :type Actor%20Object%20Reference) (OtherComp :type Primitive%20Component%20Object%20Reference) (OtherBodyIndex :type Integer))
  (bind _asthird_person_character (Utilities|Casting|CastToThirdPersonCharacter OtherActor))
  (Variables|/Game/ThirdPersonBP/Blueprints/ThirdPersonCharacter.ThirdPersonCharacter_C|SetInPortal _asthird_person_character false))

(event EventBeginPlay)

(event Collision|EventActorBeginOverlap
  (params (OtherActor :type Actor%20Object%20Reference)))

(event EventTick
  (params (DeltaSeconds :type Float%20%28single-precision%29)))

(fn ConstructionScript)